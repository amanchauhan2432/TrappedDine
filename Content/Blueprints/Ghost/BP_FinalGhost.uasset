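; BP_FinalGhost is a horror enemy ghost that chases the HorrorEngineCharacter and damages the player when its box overlaps them.
; A timeline started at BeginPlay bobs and randomly jitters the figure, and drives delayed move-to and look-at updates toward the cached character.
; Falling Health intensifies the jitter, light and dynamic material's emissive and opacity.
; At zero Health, chase and glow updates stop, while bobbing and overlap damage remain.
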(event OnComponentBeginOverlap(Box)
  (params (OverlappedComponent :type Primitive%20Component%20Object%20Reference) (OtherActor :type Actor%20Object%20Reference) (OtherComp :type Primitive%20Component%20Object%20Reference) (OtherBodyIndex :type Integer) (bFromSweep :type Boolean) (SweepResult :type Hit%20Result%20Structure%20%28by%20ref%29))
  (Utilities|Casting|CastToHorrorEngineCharacter OtherActor)
  (bind _asmaster (CallFunction|GetPlayer))
  (Default|GetDamage :self _asmaster :HorrorEvent true :DamagePoint 1.5e+02))

(event EventBeginPlay
  (bind _health (Variables|Default|GetHealth))
  (bind _returnvalue (Math|Float|MapRangeClamped _health 1e+02 0.0 2.0 1e+01))
  (bind _animation (Timeline|FigureAnimation PlayFromStart)
    (:Update
      (Transformation|SetRelativeLocation (Variables|Default|GetSampleFigure) (Math|Vector|MakeVector 0.0 0.0 (* _animation 3e+01)) false false)
      (Transformation|SetRelativeRotation (Variables|Default|GetSampleFigure) (Math|Rotator|MakeRotator (Math|Random|RandomFloatinRange (* -1.0 _returnvalue) _returnvalue) (Math|Random|RandomFloatinRange (* -1.0 _returnvalue) _returnvalue) (Math|Random|RandomFloatinRange (* -1.0 _returnvalue) _returnvalue)) false false)
      (if (not (<= (Variables|Default|GetHealth) 0.0))
        (Rendering|Components|Light|SetIntensity (Variables|Default|GetFigureLight) (Math|Float|MapRangeClamped (Variables|Default|GetHealth) 1e+02 0.0 1e+03 9e+03))
        (Rendering|Material|SetScalarParameterValue (Variables|Default|GetFigureMaterialRef) "Emissive" (Math|Float|MapRangeClamped (Variables|Default|GetHealth) 1e+02 0.0 3.0 9.0) :!class /Script/Engine.MaterialInstanceDynamic)
        (Rendering|Material|SetScalarParameterValue (Variables|Default|GetFigureMaterialRef) "Opacity" (Math|Float|MapRangeClamped (Variables|Default|GetHealth) 1e+02 0.0 0.5 1.0) :!class /Script/Engine.MaterialInstanceDynamic)
        (Utilities|FlowControl|Delay 0.1)
        (Variables|Default|GetCharacter%20Ref
          (:then
            _)
          (:else
            (bind _returnvalue_2 (Actor|GetActorOfClass "/Game/HorrorEngine/Blueprints/Core/HorrorEngineCharacter.HorrorEngineCharacter_C"))
            (Utilities|IsValid _returnvalue_2
              (:Is%20Valid
                (Variables|Default|SetCharacter%20Ref _returnvalue_2)))))
        (AI|Navigation|SimpleMovetoActor (Pawn|GetController) (Variables|Default|GetCharacter%20Ref))
        (Transformation|SetActorRotation (Math|Rotator|FindLookatRotation (Transformation|GetWorldLocation (Variables|Default|GetSampleFigure)) (Transformation|GetActorLocation (Variables|Default|GetCharacter%20Ref))))))))

(fn ConstructionScript
  (bind _returnvalue (Rendering|Material|CreateDynamicMaterialInstance (Variables|Default|GetSampleFigure) 0 "/Game/HorrorEngine/Materials/He_Noise2.He_Noise2" "None" :!class /Script/Engine.PrimitiveComponent))
  (bind _output_get (Variables|Default|SetFigureMaterialRef _returnvalue))
  (Rendering|Material|SetScalarParameterValue _output_get "Emissive" 3.0 :!class /Script/Engine.MaterialInstanceDynamic)
  (Rendering|Material|SetScalarParameterValue (Variables|Default|GetFigureMaterialRef) "Opacity" 0.5 :!class /Script/Engine.MaterialInstanceDynamic))